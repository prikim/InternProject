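; Base AI actor that chases whichever is closest of a level spline point, the player or a selected tower, all found by tag.
; A looping timer runs CheckDistances to set the target, advancing spline progress when close while following it.
; The tower pick keeps the greatest distance recorded, not the nearest.
; Tick moves a sphere to the target, smoothly yaws toward it and steps forward at zero height until within range.
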(event `self.ReceiveBeginPlay`
  (`|ExecutionSequence`
    (:`then_0`
      ;[1 0 0.3072] Get Tags
      (bind _outactors (`GameplayStatics.GetAllActorsWithTag` "Player"))
      (set `self.TargetPlayer` (`|GetArrayItem` _outactors))
      (bind _outactors_2 (`GameplayStatics.GetAllActorsWithTag` "Tower"))
      (set `self.Towers` _outactors_2)
      (bind _outactors_3 (`GameplayStatics.GetAllActorsWithTag` "Spline"))
      (bind _asspline_component (cast `SplineComponent` (`Actor.RootComponent` (`|GetArrayItem` _outactors_3)))
        (:`then`
          (set `self.LevelSpline` _asspline_component))
        (:`CastFailed`
          (`KismetSystemLibrary.PrintString` "No Spline Found" true true (struct :`R` 1.0 :`B` 0.046707 :`A` 1.0) 10.0))))
    (:`then_1`
      (`KismetSystemLibrary.K2_SetTimerDelegate` (delegate `FindClosestTarget`) 0.25 true)
      (set `self.SplineLocation` (`self.ContinueMovingAlongSpline`)))))

(event `FindClosestTarget`
  (`self.CheckDistances`))

(event `self.ReceiveTick`
  (params (DeltaSeconds :type "Float (single-precision)"))
  (`SceneComponent.K2_SetWorldLocation` (`self.Sphere`) (`self.TargetLocation`) false true)
  (`self.RotateToTarget`)
  (if (not (`self.CloseToTarget` (`self.DistanceToTarget_cm`)))
    (`self.MoveToTarget`)))

(event `MoveToTarget`
  (bind _mesh (`self.Mesh`))
  (set `self.PreviousTargetLocation` (`self.TargetLocation`))
  (`self.K2_SetActorLocation` (`KismetMathLibrary.MakeVector` (.x (+ (`SceneComponent.K2_GetComponentLocation` _mesh) (* (`SceneComponent.GetForwardVector` _mesh) (* (`self.MovementSpeed_cm`) (`GameplayStatics.GetWorldDeltaSeconds`))))) (.y (+ (`SceneComponent.K2_GetComponentLocation` _mesh) (* (`SceneComponent.GetForwardVector` _mesh) (* (`self.MovementSpeed_cm`) (`GameplayStatics.GetWorldDeltaSeconds`))))))))

(event `RotateToTarget`
  (set `self.PreviousRotation` (`SceneComponent.K2_GetComponentRotation` (`self.Mesh`)))
  (`self.K2_SetActorRotation` (`KismetMathLibrary.MakeRotator` 0.0 0.0 (.yaw (`KismetMathLibrary.RLerp` (`KismetMathLibrary.FindLookAtRotation` (`SceneComponent.K2_GetComponentLocation` (`self.Mesh`)) (`self.TargetLocation`)) (`self.PreviousRotation`) (`self.RotationSpeed`) true)))))

(fn `CheckDistances`
  (locals (IntSwitch :type Integer) (TowerDistance :type "Float (double-precision)" :default 0.0) (TowerNumber :type Integer))
  (bind _returnvalue (`KismetMathLibrary.Vector_Distance` (`self.K2_GetActorLocation` self) (`self.PlayerLocation`)))
  (`|ExecutionSequence`
    (:`then_0`
      (set `self.SplineLocation` (`self.ContinueMovingAlongSpline`))
      (set `self.PlayerLocation` (`self.K2_GetActorLocation` (`self.TargetPlayer`)))
      (for (_array_element _array_index) (`self.Towers`)
        (bind _returnvalue_2 (`self.GetDistanceTo` _array_element self))
        (if (> _returnvalue_2 (`local.TowerDistance`))
          (set `local.TowerDistance` _returnvalue_2)
          (set `local.TowerNumber` _array_index)))
      (set `self.TowerLocation` (`self.K2_GetActorLocation` (`|GetArrayItem` (`self.Towers`) (`local.TowerNumber`)))))
    (:`then_1`
      (if (< (`KismetMathLibrary.Vector_Distance` (`self.K2_GetActorLocation` self) (`self.SplineLocation`)) _returnvalue)
        (set `local.IntSwitch` 0)
        (elif (< _returnvalue (`KismetMathLibrary.Vector_Distance` (`self.K2_GetActorLocation` self) (`self.TowerLocation`)))
          (set `local.IntSwitch` 1)
          (else
            (set `local.IntSwitch` 2)))))
    (:`then_2`
      (switch `int` (`local.IntSwitch`)
        (:`Default`
          (if (`self.CloseToTarget` 300.0) :!label _label
            (set `self.SplineDistanceProgress` (+ (`self.SplineDistanceProgress`) 500.0))
            (else
              (set `self.SplineDistanceProgress` (`self.SplineDistanceProgress`))))
          (set `self.TargetLocation` (`self.SplineLocation`)))
        (:`0`
          (goto _label))
        (:`1`
          (set `self.TargetLocation` (`self.PlayerLocation`)))
        (:`2`
          (set `self.TargetLocation` (`self.TowerLocation`)))))))

(fn `CloseToTarget`
  (params (DistanceToCheck :type "Float (double-precision)"))
  (returns (StopMovement :type Boolean))
  (return (< (`KismetMathLibrary.Abs` (`KismetMathLibrary.Vector_Distance` (`SceneComponent.K2_GetComponentLocation` (`self.Mesh`)) (`self.TargetLocation`))) DistanceToCheck)))

(fn `ContinueMovingAlongSpline`
  (returns (SplineTimeLocation :type "Vector Structure"))
  (return (`SplineComponent.GetLocationAtTime` (`self.LevelSpline`) (`self.SplineDistanceProgress`) "World" false)))

(fn `UserConstructionScript`)