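; BP_Enemy is a damageable enemy actor that destroys itself when its Health runs out.
; Its Impact event takes a damage amount, prints a hit message, then subtracts the damage from Health.
; Health is checked both before and after the subtraction, and either check at zero or below destroys the actor.
; BeginPlay, overlap, Tick and the construction script contain no logic.
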(event `Impact`
  (params (`Damage Intake` :type "Float (double-precision)"))
  (`KismetSystemLibrary.PrintString` "Enemy: IM HIT")
  ;[1 1 1] Health is < 0
  (if (<= (`self.Health`) 0.0)
    (`self.K2_DestroyActor` :!label _label)
    (else
      ;[1 1 1] Health is still < 0
      (set `self.Health` (- (`self.Health`) `Damage Intake`))
      (if (<= (`self.Health`) 0.0)
        (goto _label)))))

(fn `UserConstructionScript`)